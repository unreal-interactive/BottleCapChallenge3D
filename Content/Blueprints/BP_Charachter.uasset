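; BP_Charachter is a character Blueprint that switches one skeletal mesh between a man (Ty) and a granny, both using mobile animation setups.
; ChangeCharacter sets the mesh and matching AnimBP and records the choice in NumberCharacter, defaulting to the man.
; TakeAnimFromArray plays a random one-shot animation from that character's array.
; PlayAnim prints and plays a Ty animation by index; its timed slow-motion test sequence in the event graph is unconnected.
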(event EventBeginPlay)

(event Collision|EventActorBeginOverlap
  (params (OtherActor :type Actor%20Object%20Reference)))

(event EventTick
  (params (DeltaSeconds :type Float%20%28single-precision%29)))

(fn ConstructionScript)

(fn ChangeCharacter
  (params (ABP%20number :type Integer))
  (bind _skeletalmeshcomponent (Variables|SkeletalMeshActor|GetSkeletalMeshComponent))
  (bind _skeletalmeshcomponent_2 (Variables|SkeletalMeshActor|GetSkeletalMeshComponent))
  (switch int ABP%20number
    (:Default
      (Class|SkinnedMeshComponent|SetSkeletalMesh _skeletalmeshcomponent_2 "/Game/character_TY_for_mobile/Man.Man" true :!label _label)
      (Components|SkeletalMesh|SetAnimInstanceClass _skeletalmeshcomponent "/Game/character_TY_for_mobile/ABP_TyMobile.ABP_TyMobile_C")
      (Variables|Default|SetnumberCharacter 0))
    (:0
      (goto _label))
    (:1
      (Class|SkinnedMeshComponent|SetSkeletalMesh _skeletalmeshcomponent_2 "/Game/character_granny/Granny_for_mobile.Granny_for_mobile" true)
      (Components|SkeletalMesh|SetAnimInstanceClass _skeletalmeshcomponent "/Game/character_granny/ABP_Granny_for_mobile.ABP_Granny_for_mobile_C")
      (Variables|Default|SetnumberCharacter 1))))

(fn TakeAnimfromArray
  (bind _animarrayty (Variables|Default|GetanimarrayTY))
  (bind _animarraygranny (Variables|Default|GetanimarrayGranny))
  (switch int (Variables|Default|GetnumberCharacter)
    (:Default
      (Components|Animation|PlayAnimation (Variables|SkeletalMeshActor|GetSkeletalMeshComponent) (Utilities|Array|Get(acopy) _animarrayty (Math|Random|RandomIntegerinRange 0 (Utilities|Array|LastIndex _animarrayty))) false :!label _label))
    (:0
      (goto _label))
    (:1
      (Components|Animation|PlayAnimation (Variables|SkeletalMeshActor|GetSkeletalMeshComponent) (Utilities|Array|Get(acopy) _animarraygranny (Math|Random|RandomIntegerinRange 0 (Utilities|Array|LastIndex _animarraygranny))) false))))

(fn PlayAnim
  (params (NewParam :type Integer))
  (Development|PrintString (Utilities|String|ToString(Integer) NewParam))
  (Components|Animation|PlayAnimation (Variables|SkeletalMeshActor|GetSkeletalMeshComponent) (Utilities|Array|Get(acopy) (Variables|Default|GetanimarrayTY) NewParam) false))