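; BP_SaveGame stores the game's best score as MaxScore in the "bestscore" save slot.
; Save creates a new instance of its own class, copies in the passed score and writes it to the slot.
; Load first builds and prints an instance from the passed score, then replaces it with the slot's saved object and prints that score, without returning it.
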(event Custom|Load
  (params (BestScore :type Integer))
  (bind _returnvalue (SaveGame|CreateSaveGameObject "BP_SaveGame_C"))
  (bind _output_get (Variables|Default|SetSaveGameInstance _returnvalue))
  (bind _output_get_2 (Variables|BP_SaveGame_C|SetmaxScore _output_get BestScore))
  (Development|PrintString 0 (Utilities|String|ToString(Integer) _output_get_2))
  (bind _returnvalue_2 (SaveGame|LoadGamefromSlot "bestscore"))
  (bind _asbp_save_game (Utilities|Casting|CastToBP_SaveGame _returnvalue_2))
  (bind _output_get_3 (Variables|Default|SetSaveGameInstance _asbp_save_game))
  (Development|PrintString 0 (Utilities|String|ToString(Integer) (Variables|BP_SaveGame_C|GetmaxScore _output_get_3))))

(event Custom|Save
  (params (BestScore :type Integer))
  (bind _returnvalue (SaveGame|CreateSaveGameObject "BP_SaveGame_C"))
  (bind _output_get (Variables|Default|SetSaveGameInstance _returnvalue))
  (Variables|BP_SaveGame_C|SetmaxScore _output_get BestScore)
  (SaveGame|SaveGametoSlot _output_get "bestscore"))