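; Game mode for a bottle-cap skillcheck game that runs the round loop, score, menus and music.
; BeginPlay caches the character, bottle and cap actors; each round spawns a skillcheck widget, with input gated by a DoOnce.
; Success adds score and starts another round; failure resets the props and score and shows the end menu.
; High scores save through the GameInstance, post to a leaderboard and unlock a granny character.
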(event Custom|LoadMyData
  ;[1 1 1] Load
  (bind _asbp_game_instance (Utilities|Casting|CastToBP_GameInstance (Game|GetGameInstance)))
  (bind _asbp_save_game (Default|LoadData _asbp_game_instance))
  (Utilities|IsValid _asbp_save_game
    (:Is%20Valid
      (Variables|Default|SetmaxScore (Variables|/Game/Blueprints/BP_SaveGame.BP_SaveGame_C|GetmaxScore _asbp_save_game)))))

(event Custom|Touch
  ;[1 1 1] Touch
  (Utilities|FlowControl|DoOnce true
    (:Completed
      (Default|TouchSkillcheck (Variables|Default|GetW_skillcheck)))))

(event Custom|SaveGame
  ;[1 1 1] Save
  (bind _asbp_game_instance (Utilities|Casting|CastToBP_GameInstance (Game|GetGameInstance)))
  (bind _returnvalue (SaveGame|CreateSaveGameObject "/Game/Blueprints/BP_SaveGame.BP_SaveGame_C"))
  (Variables|/Game/Blueprints/BP_SaveGame.BP_SaveGame_C|SetmaxScore _returnvalue (Variables|Default|GetmaxScore))
  (Default|SaveData _asbp_game_instance _returnvalue))

(event Custom|PLAY!
  ;[1 1 1] Touch
  ;;[1 1 1] Play!
  (bind _returnvalue (UserInterface|CreateWidget "/Game/Widgets/W_skillcheck.W_skillcheck_C"))
  (UserInterface|Viewport|AddtoViewport _returnvalue 0)
  (Variables|Default|SetW_skillcheck _returnvalue)
  (Utilities|FlowControl|DoOnce true) ; enters at Reset
)

(event Custom|NO!%20Skillcheck
  (bind _menugame (Variables|Default|GetMenuGame))
  (bind _bottle (Variables|Default|GetBottle))
  (bind _cap (Variables|Default|GetCap))
  (bind _bottle_2 (Variables|Default|GetBottle))
  (bind _staticmeshcomponent (Variables|/Script/Engine.StaticMeshActor|GetStaticMeshComponent _bottle_2))
  (bind _staticmeshcomponent_2 (Variables|/Script/Engine.StaticMeshActor|GetStaticMeshComponent _cap))
  ;[1 1 1] Touch
  (Default|FailHit (Variables|Default|GetCap))
  (Default|FailHit _bottle)
  (Physics|SetSimulatePhysics (Variables|/Script/Engine.StaticMeshActor|GetStaticMeshComponent _bottle) true)
  (Physics|SetSimulatePhysics (Variables|/Script/Engine.StaticMeshActor|GetStaticMeshComponent (Variables|Default|GetCap)) true)
  (Default|TakeAnimfromArray (Variables|Default|Getcharachter)) ; Play Random ANim
  (Utilities|FlowControl|Delay 2.0)
  (Components|Animation|SetAnimationMode (Variables|/Script/Engine.SkeletalMeshActor|GetSkeletalMeshComponent (Variables|Default|Getcharachter)) "AnimationBlueprint")
  ;;[1 1 1] Back to startPosition (bottle&cap)
  (Physics|SetSimulatePhysics _staticmeshcomponent false)
  (Physics|SetSimulatePhysics _staticmeshcomponent_2 false)
  (Transformation|SetWorldLocation _staticmeshcomponent_2 "0, 0, 0" false false)
  (Transformation|SetWorldLocation _staticmeshcomponent (Variables|Default|GetStartLoc_Bottle) false false)
  (Transformation|SetWorldRotation _staticmeshcomponent "0, 0, 0" false false)
  (CallFunction|SetStartPosCAP)
  (Default|ShowVisible _menugame)
  (Default|ScoreEnd _menugame (Variables|Default|Getscore))
  (CallFunction|CheckOpenCharachter)
  (Variables|Default|Setscore 0)
  (Default|EditScore (Variables|Default|GetSCORE_WIdget) (Utilities|Text|ToText(String) (Utilities|String|Append "Score: " (Utilities|String|ToString(Integer) (Variables|Default|Getscore))))))

(event Custom|Yes!%20Skillcheck
  (bind _cap (Variables|Default|GetCap))
  ;[1 1 1] Touch
  (Default|SuccessHit _cap)
  (Default|SuccessHit (Variables|Default|GetBottle))
  (Physics|SetSimulatePhysics (Variables|/Script/Engine.StaticMeshActor|GetStaticMeshComponent _cap) true)
  (Development|PrintString "Physic ON!")
  (Default|TakeAnimfromArray (Variables|Default|Getcharachter)) ; Play Random ANim
  (Math|Integer|IncrementInt (Variables|Default|Getscore)
    (:%20%20
      (Utilities|FlowControl|Delay 2.0)
      (Components|Animation|SetAnimationMode (Variables|/Script/Engine.SkeletalMeshActor|GetSkeletalMeshComponent (Variables|Default|Getcharachter)) "AnimationBlueprint")
      ;;[1 1 1] back to startPosition (cap)
      (CallFunction|SetStartPosCAP)
      ;;[1 1 1] Score
      (CallFunction|SetBestScore)
      (Default|EditScore (Variables|Default|GetSCORE_WIdget) (Utilities|Text|ToText(String) (Utilities|String|Append "Score: " (Utilities|String|ToString(Integer) (Variables|Default|Getscore)))))
      (CallFunction|CheckOpenCharachter)
      (CallFunction|PLAY!) ; PlaySkillcheck!
    )))

(event EventBeginPlay
  ;[1 1 1] BeginPlay
  (bind _returnvalue (UserInterface|CreateWidget "/Game/Widgets/W_MainMenu.W_MainMenu_C"))
  (bind _output_get (Variables|Default|SetMainMenu _returnvalue))
  (UserInterface|Viewport|AddtoViewport _output_get 0)
  (bind _returnvalue_2 (UserInterface|CreateWidget "/Game/Widgets/W_MenuGame.W_MenuGame_C"))
  (bind _output_get_2 (Variables|Default|SetMenuGame _returnvalue_2))
  (UserInterface|Viewport|AddtoViewport _output_get_2 0)
  (Widget|SetVisibility _output_get_2 "Hidden")
  (bind _outactors (Actor|GetAllActorsOfClass "/Script/Engine.CameraActor"))
  (Components|Activation|SetAutoActivate (Variables|/Script/Engine.CameraActor|GetCameraComponent (Utilities|Array|Get(acopy) _outactors)) true)
  (bind _outactors_2 (Actor|GetAllActorsOfClass "/Game/Blueprints/BP_Charachter.BP_Charachter_C"))
  (Variables|Default|Setcharachter (Utilities|Array|Get(acopy) _outactors_2))
  (Input|EnableInput (Game|GetPlayerController 0))
  (bind _outactors_3 (Actor|GetAllActorsOfClass "/Game/Blueprints/BP_Bottle.BP_Bottle_C"))
  (bind _output_get_3 (Variables|Default|SetBottle (Utilities|Array|Get(acopy) _outactors_3)))
  (Variables|Default|SetStartLoc_Bottle (Transformation|GetActorLocation _output_get_3))
  (bind _outactors_4 (Actor|GetAllActorsOfClass "/Game/Blueprints/BP_Cap.BP_Cap_C"))
  (Variables|Default|SetCap (Utilities|Array|Get(acopy) _outactors_4))
  (bind _returnvalue_3 (UserInterface|CreateWidget "/Game/Widgets/W_Ad_banner.W_Ad_banner_C"))
  (UserInterface|Viewport|AddtoViewport _returnvalue_3 1)
  (bind _returnvalue_4 (Audio|CreateSound2D "/Game/Audio/Komiku_-_09_-_Glouglou_Cue.Komiku_-_09_-_Glouglou_Cue" 0.3 1.0 0.0 0))
  (bind _output_get_4 (Variables|Default|SetSound _returnvalue_4))
  (Audio|Components|Audio|Play _output_get_4 0.0)
  (CallFunction|SetStartPosCAP)
  (Physics|SetSimulatePhysics (Variables|/Script/Engine.StaticMeshActor|GetStaticMeshComponent (Variables|Default|GetCap)) true)
  (Utilities|FlowControl|Delay 0.2)
  (Development|PrintString (Utilities|String|ToString(Vector) (Transformation|GetWorldLocation (Variables|/Script/Engine.StaticMeshActor|GetStaticMeshComponent (Variables|Default|GetCap)))))
  (CallFunction|CheckOpenCharachter))

(event Input|KeyboardEvents|Q
  (params (Key :type Key%20Structure))
  ;[1 1 1] Touch
  (:Released
    (Utilities|FlowControl|DoOnce true
      (:Completed
        (Default|TouchSkillcheck (Variables|Default|GetW_skillcheck))))))

(event Input|KeyboardEvents|1
  (params (Key :type Key%20Structure))
  ;[1 1 1] Touch
  (:Released
    (Utilities|FlowControl|DoOnce true
      (:Completed
        (Default|TouchSkillcheck (Variables|Default|GetW_skillcheck))))))

(fn ConstructionScript)

(fn CreateWidget
  (bind _returnvalue (UserInterface|CreateWidget "/Game/Widgets/UI_GameButton1.UI_GameButton1_C" (Game|GetPlayerController 0)))
  (bind _output_get (Variables|Default|SetSCORE_WIdget _returnvalue))
  (UserInterface|Viewport|AddtoViewport _output_get 0))

(fn Reset)

(fn SetBestScore
  (if (> (Variables|Default|Getscore) (Variables|Default|GetmaxScore))
    (bind _output_get (Variables|Default|SetmaxScore (Variables|Default|Getscore)))
    (Default|EditBest (Variables|Default|GetSCORE_WIdget) (Utilities|Text|ToText(Integer) (Variables|Default|Getscore)))
    (CallFunction|SaveGame)
    (Class|LeaderboardBlueprintLibrary|WriteLeaderboardInteger (Game|GetPlayerController 0) "Caps" _output_get)))

(fn SetStartPosCAP
  (bind _cap (Variables|Default|GetCap))
  (bind _startloc_bottle (Variables|Default|GetStartLoc_Bottle))
  (bind _staticmeshcomponent (Variables|/Script/Engine.StaticMeshActor|GetStaticMeshComponent _cap))
  (Physics|SetSimulatePhysics _staticmeshcomponent false)
  (Development|PrintString "Physic OFF!")
  (Transformation|SetWorldLocation _staticmeshcomponent (Math|Vector|MakeVector (.x _startloc_bottle) (.y _startloc_bottle) (.z _startloc_bottle)) false false)
  (Transformation|SetWorldRotation _staticmeshcomponent "0, 0, 0" false false))

(fn PlayOffSound
  (bind _sound (Variables|Default|GetSound))
  (if (Variables|Default|Getissound?)
    (Class|AudioComponent|SetPaused _sound true)
    (Variables|Default|Setissound? false)
    (else
      (Class|AudioComponent|SetPaused _sound false)
      (Variables|Default|Setissound? true))))

(fn CheckOpenCharachter
  (if (>= (Variables|Default|GetmaxScore) 30)
    (Default|Opengranny (Variables|Default|GetMainMenu))))

(fn ShowLeaderBoard)